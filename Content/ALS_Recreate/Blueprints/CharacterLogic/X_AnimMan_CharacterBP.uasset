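; AnimMan character Blueprint in an ALS recreation that supplies camera reference points through interface functions, with an empty event graph.
; Third person trace parameters use a left or right shoulder mesh socket, chosen by RightShoulder, with a fixed radius on the Visibility channel.
; The third person pivot averages the head and root socket locations with actor rotation, while first person uses the FP_Camera socket.
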(fn `BPI_Get_FP_CameraTarget`
  (returns (`Return Value` :type "Vector Structure"))
  ;[1 1 1] Get the camera position in the first person view.
  (return (`SceneComponent.GetSocketLocation` (`self.Mesh`) "FP_Camera")))

(fn `BPI_Get_TP_PivotTarget`
  (returns (`Return Value` :type "Transform Structure"))
  (bind _mesh (`self.Mesh`))
  ;[0 1 0.5232] The anchor position of the character in the third person view.
  (return (`KismetMathLibrary.MakeTransform` (`KismetMathLibrary.GetVectorArrayAverage` (`|MakeArray` (`SceneComponent.GetSocketLocation` _mesh "head") (`SceneComponent.GetSocketLocation` _mesh "root"))) (`self.K2_GetActorRotation`))))

(fn `BPI_Get_TP_TraceParams`
  (returns (`Trace Origin` :type "Vector Structure") (`Trace Radius` :type "Float (double-precision)") (`Trace Channel` :type "ETraceTypeQuery Enum"))
  ;[0.2721 1 0] Get camera position of right or left shoulder in the third person view.
  (if (`self.RightShoulder`)
    (return (`SceneComponent.GetSocketLocation` (`self.Mesh`) "TP_CameraTrace_R") 10.0 "TraceTypeQuery1")
    (else
      (return (`SceneComponent.GetSocketLocation` (`self.Mesh`) "TP_CameraTrace_L") 10.0 "TraceTypeQuery1"))))

(fn `UserConstructionScript`
  (`parent.UserConstructionScript`))