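; X_BaseCharacterBP is a base character Blueprint in an ALS (Advanced Locomotion System) recreation that supplies camera data through BPI getter functions.
; It returns first and third person FOV with the shoulder side, and the FP_Camera mesh socket location for first person.
; The actor's transform serves as the third person pivot, and its location as the origin of a small-radius Visibility trace.
; The event graph and construction script contain no logic.
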(fn `BPI_Get_CameraParameters`
  (returns (`TP FOV` :type "Float (double-precision)") (`FP FOV` :type "Float (double-precision)") (RightShoulder :type Boolean))
  (return (`self.ThirdPersonFOV`) (`self.FirstPersonFOV`) (`self.RightShoulder`)))

(fn `BPI_Get_FP_CameraTarget`
  (returns (`Return Value` :type "Vector Structure"))
  (return (`SceneComponent.GetSocketLocation` (`self.Mesh`) "FP_Camera")))

(fn `BPI_Get_TP_PivotTarget`
  (returns (`Return Value` :type "Transform Structure"))
  (return (`self.GetTransform`)))

(fn `BPI_Get_TP_TraceParams`
  (returns (`Trace Origin` :type "Vector Structure") (`Trace Radius` :type "Float (double-precision)") (`Trace Channel` :type "ETraceTypeQuery Enum"))
  (return (`self.K2_GetActorLocation`) 10.0 "TraceTypeQuery1"))

(fn `UserConstructionScript`)