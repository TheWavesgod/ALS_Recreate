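; ALS-style player camera manager that replaces the default camera update for pawns tagged X_Character with a custom third/first-person camera.
; Pivot, first-person target, FOV and trace settings come from the pawn via interface calls; curves from a camera behaviour AnimBP drive lags, offsets and blend weights.
; The pivot follows with per-axis lag in camera-yaw space, then gets offset, and a sphere trace pulls the camera out of walls.
; Debug pivot shapes always draw.
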(event `OnPossess`
  (params (NewPawn :type "Pawn Object Reference"))
  (set `self.ControlledPawn` NewPawn)
  (bind _asx_player_camera_behaviour (cast `/Game/ALS_Recreate/Blueprints/CameraSystem/X_PlayerCameraBehaviour` (`SkeletalMeshComponent.GetAnimInstance` (`self.CameraBehaviour`))))
  (set `/Game/ALS_Recreate/Blueprints/CameraSystem/X_PlayerCameraBehaviour.PlayerController` (`self.GetOwningPlayerController`) _asx_player_camera_behaviour)
  (set `/Game/ALS_Recreate/Blueprints/CameraSystem/X_PlayerCameraBehaviour.ControlledPawn` (`self.ControlledPawn`) _asx_player_camera_behaviour))

(fn `BlueprintUpdateCamera`
  (params (CameraTarget :type "Actor Object Reference"))
  (returns (NewCameraLocation :type "Vector Structure") (NewCameraRotation :type "Rotator Structure") (NewCameraFOV :type "Float (single-precision)") (ReturnValue :type Boolean))
  ;[1 1 1] Determining if the controlled pawn is the X_Character.
  (if (`self.ActorHasTag` CameraTarget "X_Character")
    (bind (_location _rotation _fov) (`self.CustomCameraBehaviour`))
    (return _location _rotation _fov true)
    (else
      (bind (_newcameralocation _newcamerarotation _newcamerafov _returnvalue) (`parent.BlueprintUpdateCamera` (`local.CameraTarget`)))
      (return _newcameralocation _newcamerarotation _newcamerafov _returnvalue))))

(fn `CalculateAxisLndependentLag`
  (params (CurrentLocation :type "Vector Structure") (TargetLocation :type "Vector Structure") (CameraRotation :type "Rotator Structure") (LagSpeed :type "Vector Structure"))
  (returns (ReturnValue :type "Vector Structure"))
  (locals (CameraRotationYaw :type "Rotator Structure"))
  (bind _returnvalue (`GameplayStatics.GetWorldDeltaSeconds`))
  (bind (_camerarotation_roll _camerarotation_pitch _camerarotation_yaw) (`KismetMathLibrary.BreakRotator` (`local.CameraRotation`)))
  (bind (_lagspeed_x _lagspeed_y _lagspeed_z) (`KismetMathLibrary.BreakVector` (`local.LagSpeed`)))
  (bind _camerarotationyaw (`local.CameraRotationYaw`))
  (bind (_returnvalue_x _returnvalue_y _returnvalue_z) (`KismetMathLibrary.BreakVector` (`KismetMathLibrary.LessLess_VectorRotator` (`local.TargetLocation`) _camerarotationyaw)))
  (bind (_returnvalue_x_2 _returnvalue_y_2 _returnvalue_z_2) (`KismetMathLibrary.BreakVector` (`KismetMathLibrary.LessLess_VectorRotator` (`local.CurrentLocation`) _camerarotationyaw)))
  (set `local.CameraRotationYaw` (`KismetMathLibrary.MakeRotator` 0.0 0.0 _camerarotation_yaw))
  (return (`KismetMathLibrary.GreaterGreater_VectorRotator` (`KismetMathLibrary.MakeVector` (`KismetMathLibrary.FInterpTo` _returnvalue_x_2 _returnvalue_x _returnvalue _lagspeed_x) (`KismetMathLibrary.FInterpTo` _returnvalue_y_2 _returnvalue_y _returnvalue _lagspeed_y) (`KismetMathLibrary.FInterpTo` _returnvalue_z_2 _returnvalue_z _returnvalue _lagspeed_z)) (`local.CameraRotationYaw`))))

(fn `CustomCameraBehaviour`
  (returns (Location :type "Vector Structure") (Rotation :type "Rotator Structure") (FOV :type "Float (double-precision)"))
  (locals (TPPivotTarget :type "Transform Structure") (FPTarget :type "Vector Structure" :default (0.0 0.0 0.0)) (TPFOV :type "Float (double-precision)" :default 0.0) (FPFOV :type "Float (double-precision)" :default 0.0) (RightShoulder :type Boolean :default false))
  (bind _targetcamerarotation (`self.TargetCameraRotation`))
  (bind _smoothtargetpivot_location (`KismetMathLibrary.BreakTransform` (`self.SmoothTargetPivot`)))
  (bind _tppivottarget_location (`KismetMathLibrary.BreakTransform` (`local.TPPivotTarget`)))
  (bind _smoothtargetpivot_location_2 (`KismetMathLibrary.BreakTransform` (`self.SmoothTargetPivot`)))
  (bind _smoothtargetpivot_location_3 (`KismetMathLibrary.BreakTransform` (`self.SmoothTargetPivot`)))
  (bind _tppivottarget_location_2 (`KismetMathLibrary.BreakTransform` (`local.TPPivotTarget`)))
  (bind _smoothtargetpivot_location_4 (`KismetMathLibrary.BreakTransform` (`self.SmoothTargetPivot`)))
  (bind _smoothtargetpivot_location_5 (`KismetMathLibrary.BreakTransform` (`self.SmoothTargetPivot`)))
  (bind (_tppivottarget_location_3 _tppivottarget_rotation _tppivottarget_scale) (`KismetMathLibrary.BreakTransform` (`local.TPPivotTarget`)))
  (bind _tppivottarget_location_4 (`KismetMathLibrary.BreakTransform` (`local.TPPivotTarget`)))
  (bind _smoothtargetpivot_location_6 (`KismetMathLibrary.BreakTransform` (`self.SmoothTargetPivot`)))
  (bind (_smoothtargetpivot_location_7 _smoothtargetpivot_rotation) (`KismetMathLibrary.BreakTransform` (`self.SmoothTargetPivot`)))
  (`|ExecutionSequence`
    (:`then_0`
      ;[1 1 1] Get the info from Character blueprint using the BPI
      (bind _return_value (message `/Game/ALS_Recreate/Blueprints/Interfaces/X_Camera_BPI.BPI_Get_TP_PivotTarget` (`self.ControlledPawn`)))
      (set `local.TPPivotTarget` _return_value)
      (bind _return_value_2 (message `/Game/ALS_Recreate/Blueprints/Interfaces/X_Camera_BPI.BPI_Get_FP_CameraTarget` (`self.ControlledPawn`)))
      (set `local.FPTarget` _return_value_2)
      (bind (_tp_fov _fp_fov _rightshoulder) (message `/Game/ALS_Recreate/Blueprints/Interfaces/X_Camera_BPI.BPI_Get_CameraParameters` (`self.ControlledPawn`)))
      (set `local.TPFOV` _tp_fov)
      (set `local.FPFOV` _fp_fov)
      (set `local.RightShoulder` _rightshoulder))
    (:`then_1`
      ;[1 1 1] Let Camera Chase the PlayerController's rotation.
      (set `self.TargetCameraRotation` (`KismetMathLibrary.RLerp` (`KismetMathLibrary.RInterpTo` (`self.GetCameraRotation`) (`Controller.GetControlRotation` (`self.GetOwningPlayerController`)) (`GameplayStatics.GetWorldDeltaSeconds`) (`self.GetCameraBehaviourCurvesValue` "RotationLagSpeed")) (`self.DebugViewRotation`) (`self.GetCameraBehaviourCurvesValue` "Override_Debug") true)))
    (:`then_2`
      ;[1 1 1] The pivot target transform information obtained from the character blueprint is stored in the player camera manager through a transitional process, then further numerical changes are applied based on the pivot target point, primarily focused on the position.
      (set `self.SmoothTargetPivot` (`KismetMathLibrary.MakeTransform` (`self.CalculateAxisLndependentLag` _smoothtargetpivot_location_5 _tppivottarget_location_4 (`self.TargetCameraRotation`) (`KismetMathLibrary.MakeVector` (`self.GetCameraBehaviourCurvesValue` "PivotLagSpeed_X") (`self.GetCameraBehaviourCurvesValue` "PivotLagSpeed_Y") (`self.GetCameraBehaviourCurvesValue` "PivotLagSpeed_Z"))) _tppivottarget_rotation _tppivottarget_scale)))
    (:`then_3`
      ;[1 1 1] Comment
      (set `self.PivotLocation` (+ _smoothtargetpivot_location_6 (* (`KismetMathLibrary.GetForwardVector` _smoothtargetpivot_rotation) (`self.GetCameraBehaviourCurvesValue` "PivotOffset_X")) (* (`KismetMathLibrary.GetRightVector` _smoothtargetpivot_rotation) (`self.GetCameraBehaviourCurvesValue` "PivotOffset_Y")) (* (`KismetMathLibrary.GetUpVector` _smoothtargetpivot_rotation) (`self.GetCameraBehaviourCurvesValue` "PivotOffset_Z")))))
    (:`then_4`
      ;[1 1 1] Building upon the previous pivot point, we made additional numerical increases, resulting in the desired camera position.
      (set `self.TargetCameraLocation` (`KismetMathLibrary.VLerp` (+ (`self.PivotLocation`) (* (`KismetMathLibrary.GetForwardVector` _targetcamerarotation) (`self.GetCameraBehaviourCurvesValue` "CameraOffset_X")) (* (`KismetMathLibrary.GetRightVector` _targetcamerarotation) (`self.GetCameraBehaviourCurvesValue` "CameraOffset_Y")) (* (`KismetMathLibrary.GetUpVector` _targetcamerarotation) (`self.GetCameraBehaviourCurvesValue` "CameraOffset_Z"))) (+ _smoothtargetpivot_location (`self.DebugViewOffset`)) (`self.GetCameraBehaviourCurvesValue` "Override_Debug"))))
    (:`then_5`
      ;[1 1 1] Shpere trace from the character's starting point to the target camera location to prevent camera overlap with walls, and update the target camera location.
      (bind (_trace_origin _trace_radius _trace_channel) (message `/Game/ALS_Recreate/Blueprints/Interfaces/X_Camera_BPI.BPI_Get_TP_TraceParams` (`self.ControlledPawn`)))
      (bind _outhit (`KismetSystemLibrary.SphereTraceSingle` _trace_origin (`self.TargetCameraLocation`) _trace_radius _trace_channel))
      (bind (_bblockinghit _binitialoverlap _time _distance _location _impactpoint _normal _impactnormal _physmat _hitactor _hitcomponent _hitbonename _bonename _hititem _elementindex _faceindex _tracestart _traceend) (`GameplayStatics.BreakHitResult` _outhit))
      (if (and _bblockinghit (not _binitialoverlap))
        (set `self.TargetCameraLocation` (+ (- _location _traceend) (`self.TargetCameraLocation`)))))
    (:`then_6`
      ;[1 1 1] Debug
      (if true
        (`KismetSystemLibrary.DrawDebugSphere` _tppivottarget_location 16.0 8 (struct :`G` 1.0 :`B` 0.041187 :`A` 1.0) 0.0 0.5)
        (`KismetSystemLibrary.DrawDebugSphere` _smoothtargetpivot_location_2 16.0 8 (struct :`R` 0.942708 :`G` 0.535598 :`A` 1.0) 0.0 0.5)
        (`KismetSystemLibrary.DrawDebugSphere` (`self.PivotLocation`) 16.0 8 (struct :`R` 0.019431 :`G` 0.575879 :`B` 0.942708 :`A` 1.0) 0.0 0.5)
        (`KismetSystemLibrary.DrawDebugLine` _smoothtargetpivot_location_4 _tppivottarget_location_2 (struct :`R` 1.0 :`G` 0.808392 :`A` 1.0) 0.0 1.0)
        (`KismetSystemLibrary.DrawDebugLine` (`self.PivotLocation`) _smoothtargetpivot_location_3 (struct :`G` 0.306107 :`B` 1.0 :`A` 1.0) 0.0 1.0)))
    (:`then_7`
      ;[1 1 1] Return value of Camera
      (return (.location (`KismetMathLibrary.TLerp` (`KismetMathLibrary.TLerp` (`KismetMathLibrary.MakeTransform` (`self.TargetCameraLocation`) (`self.TargetCameraRotation`)) (`KismetMathLibrary.MakeTransform` (`local.FPTarget`) (`self.TargetCameraRotation`)) (`self.GetCameraBehaviourCurvesValue` "Weight_FirstPerson")) (`KismetMathLibrary.MakeTransform` (`self.DebugViewOffset`) (`self.DebugViewRotation`)) (`self.GetCameraBehaviourCurvesValue` "Override_Debug"))) (.rotation (`KismetMathLibrary.TLerp` (`KismetMathLibrary.TLerp` (`KismetMathLibrary.MakeTransform` (`self.TargetCameraLocation`) (`self.TargetCameraRotation`)) (`KismetMathLibrary.MakeTransform` (`local.FPTarget`) (`self.TargetCameraRotation`)) (`self.GetCameraBehaviourCurvesValue` "Weight_FirstPerson")) (`KismetMathLibrary.MakeTransform` (`self.DebugViewOffset`) (`self.DebugViewRotation`)) (`self.GetCameraBehaviourCurvesValue` "Override_Debug"))) (`KismetMathLibrary.Lerp` (`local.TPFOV`) (`local.FPFOV`) (`self.GetCameraBehaviourCurvesValue` "Weight_FirstPerson"))))))

(fn `GetCameraBehaviourCurvesValue`
  (params (Curves :type Name))
  (returns (ReturnValue :type "Float (double-precision)"))
  (bind _returnvalue (`SkeletalMeshComponent.GetAnimInstance` (`self.CameraBehaviour`)))
  ;[1 1 1] Get Curves value from Camera Anim Blueprint
  (`/Engine/EditorBlueprintResources/StandardMacros.IsValid` _returnvalue
    (:`Is Valid`
      (return (`AnimInstance.GetCurveValue` _returnvalue Curves)))
    (:`Is Not Valid`
      (return 0.0))))

(fn `UserConstructionScript`)